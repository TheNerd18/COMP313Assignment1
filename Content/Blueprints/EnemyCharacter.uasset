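; Zombie enemy Character that attacks the player, takes bullet damage and drops ammo on death.
; Construction sets health and randomly picks walk or sprint speed.
; Tick uses Delays to throttle a square X/Y proximity check on the player, calling TakeDamage when close.
; DamageTaken shows a hit marker and lowers health, or on a lethal hit plays the death animation, destroys the capsule, spawns ammo and increases score.
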(event `self.ReceiveTick`
  (params (DeltaSeconds :type "Float (single-precision)"))
  (`self.CheckAttack`)
  (`KismetSystemLibrary.Delay` 1.5)
  (`self.CheckAttack`)
  (if (`self.isAttacking`)
    (bind _asfirst_person_character (cast `/Game/FirstPersonBP/Blueprints/FirstPersonCharacter` (`GameplayStatics.GetPlayerCharacter` 0)))
    (`/Game/FirstPersonBP/Blueprints/FirstPersonCharacter.TakeDamage` _asfirst_person_character)
    (`KismetSystemLibrary.Delay` 3.0)))

(fn `CheckAttack`
  (bind _output_get (set `self.EnemyLocation` (`SceneComponent.K2_GetComponentLocation` (`self.Mesh`))))
  (bind _output_get_2 (set `self.PlayerLocation` (`SceneComponent.K2_GetComponentLocation` (`Actor.RootComponent` (`GameplayStatics.GetPlayerCharacter` 0)))))
  (bind _x (.x (- _output_get _output_get_2)))
  (bind _y (.y (- _output_get _output_get_2)))
  (if (< _x 125.0)
    (if (< _y 125.0)
      (if (> _x -125.0)
        (if (> _y -125.0)
          (set `self.isAttacking` true)
          (else
            (set `self.isAttacking` false :!label _label)))
        (else
          (goto _label)))
      (else
        (goto _label)))
    (else
      (goto _label))))

(fn `Damage Taken`
  (bind _returnvalue (`|CreateWidget` "/Game/FirstPersonBP/UI/HitMarker.HitMarker_C"))
  (`UserWidget.AddToViewport` _returnvalue 0)
  (if (<= (`self.health`) (`self.BulletDamage`))
    (`SkeletalMeshComponent.PlayAnimation` (`self.Mesh`) "/Game/Blueprints/Animations/ZombieAnimations/Zombie_Death.Zombie_Death" false)
    (`self.Stop Movement`)
    (`self.DropItem`)
    (bind _asfirst_person_character (cast `/Game/FirstPersonBP/Blueprints/FirstPersonCharacter` (`GameplayStatics.GetPlayerCharacter` 0)))
    (`/Game/FirstPersonBP/Blueprints/FirstPersonCharacter.IncreaseScore` _asfirst_person_character)
    (else
      (set `self.health` (- (`self.health`) (`self.BulletDamage`))))))

(fn `DropItem`
  (`|SpawnActorFromClass` "/Game/Blueprints/DropItems/AmmoDrop.AmmoDrop_C" (`self.deathLocation `) "Undefined" "OverrideRootScale" null null))

(fn `Stop Movement`
  (set `self.deathLocation ` (`KismetMathLibrary.Conv_VectorToTransform` (`SceneComponent.K2_GetComponentLocation` (`self.CapsuleComponent`))))
  (`ActorComponent.K2_DestroyComponent` (`self.CapsuleComponent`)))

(fn `UserConstructionScript`
  (set `self.health` 100)
  (if (<= (`KismetMathLibrary.RandomFloatInRange` 0.0 1.0) 0.5)
    (set `CharacterMovementComponent.MaxWalkSpeed` (`self.WalkSpeed`) (`self.CharacterMovement`))
    (else
      (set `CharacterMovementComponent.MaxWalkSpeed` (`self.SprintSpeed`) (`self.CharacterMovement`)))))