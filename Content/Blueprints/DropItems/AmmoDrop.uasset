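; AmmoDrop is a dropped item that gives ammo to the first-person character when it overlaps the drop's Cube.
; On overlap it first destroys an indexed entry in the character's PickUpItems array, then calls PickUpAmmo on the GunParent held in the Gun child actor component.
; It then plays a 2D pop sound and destroys itself, which only happens if the gun cast succeeds.
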(event `self.Cube.OnComponentBeginOverlap`
  (params (OverlappedComponent :type "PrimitiveComponent Object Reference") (OtherActor :type "Actor Object Reference") (OtherComp :type "PrimitiveComponent Object Reference") (OtherBodyIndex :type Integer) (bFromSweep :type Boolean) (SweepResult :type "HitResult Structure (by ref)"))
  (bind _asfirst_person_character (cast `/Game/FirstPersonBP/Blueprints/FirstPersonCharacter` OtherActor))
  (`self.K2_DestroyActor` (`|GetArrayItem` (`/Game/FirstPersonBP/Blueprints/FirstPersonCharacter.PickUpItems` _asfirst_person_character) (`self.index`)))
  (bind _asgun_parent (cast `/Game/FirstPersonBP/Blueprints/Guns/GunParent` (`ChildActorComponent.ChildActor` (`/Game/FirstPersonBP/Blueprints/FirstPersonCharacter.Gun` _asfirst_person_character))))
  (`/Game/FirstPersonBP/Blueprints/Guns/GunParent.pickUpAmmo` _asgun_parent)
  (`GameplayStatics.PlaySound2D` "/Game/Assets/Pop__Minecraft_Sound__-_Sound_Effect_for_editing.Pop__Minecraft_Sound__-_Sound_Effect_for_editing" 1.0 1.0 0.0 null null)
  (`self.K2_DestroyActor`))

(fn `UserConstructionScript`)